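; Flagpole actor that moves its flag and awards Mario a score bonus when he touches it.
; A Box overlap from a Mario-owned component slides the Plane over one second to a height offset below the Flag component's relative Z.
; The FlagRaised boolean limits the bonus to the first touch, while the move is requested on every overlap.
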(event `self.ReceiveTick`
  (params (DeltaSeconds :type "Float (single-precision)")))

(event `self.Box.OnComponentBeginOverlap`
  (params (OverlappedComponent :type "PrimitiveComponent Object Reference") (OtherActor :type "Actor Object Reference") (OtherComp :type "PrimitiveComponent Object Reference") (OtherBodyIndex :type Integer) (bFromSweep :type Boolean) (SweepResult :type "HitResult Structure (by ref)"))
  (bind _plane (`self.Plane`))
  (bind _asmario (cast `/Game/ThirdPersonBP/Blueprints/Mario` (`ActorComponent.GetOwner` OtherComp)))
  (`/Engine/EditorBlueprintResources/StandardMacros.IsValid` _asmario
    (:`Is Valid`
      (`KismetSystemLibrary.MoveComponentTo` _plane (`KismetMathLibrary.MakeVector` (.x (`SceneComponent.RelativeLocation` _plane)) (.y (`SceneComponent.RelativeLocation` _plane)) (- (.z (`SceneComponent.RelativeLocation` (`self.Flag`))) 600.0)) (struct :`Pitch` 90.0 :`Roll` 90.0) false false 1.0)
      (if (not (`self.FlagRaised`))
        (set `/Game/ThirdPersonBP/Blueprints/Mario.Score` (+ (`/Game/ThirdPersonBP/Blueprints/Mario.Score` _asmario) 1000) _asmario)
        (set `self.FlagRaised` true)))))

(fn `UserConstructionScript`)