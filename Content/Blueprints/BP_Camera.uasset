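; BP_Camera is a camera actor that follows FollowTarget in X and Y while keeping its own height.
; Each Tick, UpdateCameraPosition smooths toward the target with VInterpTo, using LeftBound rather than its current X as the interpolation start.
; LeftBound begins at StartingPosition and updates only while the camera's X exceeds that value, limiting drift below the start.
; SetLeftBound is an empty stub.
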(event `self.ReceiveBeginPlay`
  (set `self.LeftBound` (`self.Starting Position`)))

(event `self.ReceiveTick`
  (params (DeltaSeconds :type "Float (single-precision)"))
  (bind _returnvalue_x (`KismetMathLibrary.BreakVector` (`self.K2_GetActorLocation`)))
  (`self.UpdateCameraPosition`)
  (if (> _returnvalue_x (`self.Starting Position`))
    (set `self.LeftBound` _returnvalue_x)))

(fn `Set Left Bound`)

(fn `UpdateCameraPosition`
  (bind (_returnvalue_x _returnvalue_y _returnvalue_z) (`KismetMathLibrary.BreakVector` (`self.K2_GetActorLocation`)))
  (bind (_returnvalue_x_2 _returnvalue_y_2 _returnvalue_z_2) (`KismetMathLibrary.BreakVector` (`self.K2_GetActorLocation`)))
  (bind (_returnvalue_x_3 _returnvalue_y_3) (`KismetMathLibrary.BreakVector` (`self.K2_GetActorLocation` (`self.FollowTarget`))))
  (`self.K2_SetActorLocation` (`KismetMathLibrary.VInterpTo` (`KismetMathLibrary.MakeVector` (`self.LeftBound`) _returnvalue_y _returnvalue_z) (`KismetMathLibrary.MakeVector` _returnvalue_x_3 _returnvalue_y_3 _returnvalue_z_2) (`GameplayStatics.GetWorldDeltaSeconds`) 8.0)))

(fn `UserConstructionScript`)