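; Koopa-style tortoise enemy for a Mario-like game that walks back and forth, flipping direction on Collision_BP markers.
; Mario landing on top or touching the side triggers a timed shell mode that squashes the mesh and boosts speed; side touches send it sliding.
; Body contact damages Mario, or kills the tortoise under star power.
; Delayed collision-channel toggles on itself, other tortoises, Goombas and plants provide brief invulnerability windows.
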(event `self.ReceiveTick`
  (params (DeltaSeconds :type "Float (single-precision)"))
  ;[1 1 1] Movement
  (if (`self.CanMove`)
    (`self.K2_AddActorWorldOffset` (`KismetMathLibrary.MakeVector` (* (`self.MoveSpeed`) DeltaSeconds (`self.Direction`))))
    (if (== (`self.Direction`) -1.0)
      (`self.K2_SetActorRotation` :`self` self)
      (else
        (`self.K2_SetActorRotation` self (struct :`Yaw` 180.0) false)))))

(event `ShellMode`
  (bind _tortoisemesh (`self.TortoiseMesh`))
  (bind (_returnvalue_x _returnvalue_y _returnvalue_z) (`KismetMathLibrary.BreakVector` (`SceneComponent.K2_GetComponentScale` _tortoisemesh)))
  ;[1 1 1] Shell Mode
  (`GameplayStatics.PlaySoundAtLocation` "/Game/Audio/Squish_Cue.Squish_Cue" (`self.K2_GetActorLocation` self) (struct) 1.0 1.0 0.0 null null null)
  (set `self.CanMove` false)
  (`SceneComponent.SetWorldScale3D` _tortoisemesh (`KismetMathLibrary.MakeVector` 0.2 _returnvalue_y _returnvalue_z))
  (set `self.IsShell` true)
  (set `self.MoveSpeed` (* (`self.MoveSpeed`) (`self.MoveSpeedMultiplier`)))
  (`KismetSystemLibrary.Delay` (`self.ShellModeDuration`))
  (`SceneComponent.SetWorldScale3D` _tortoisemesh (`KismetMathLibrary.MakeVector` 0.5 _returnvalue_y _returnvalue_z))
  (set `self.CanMove` true)
  (set `self.IsShell` false)
  (set `self.MoveSpeed` (/ (`self.MoveSpeed`) (`self.MoveSpeedMultiplier`))))

(event `self.DamageCollision.OnComponentBeginOverlap`
  (params (OverlappedComponent :type "PrimitiveComponent Object Reference") (OtherActor :type "Actor Object Reference") (OtherComp :type "PrimitiveComponent Object Reference") (OtherBodyIndex :type Integer) (bFromSweep :type Boolean) (SweepResult :type "HitResult Structure (by ref)"))
  ;[1 1 1] Death/ Damage Player + Change Direction
  (cast `/Game/Blueprints/Collision_BP` OtherActor
    (:`then`
      (set `self.Direction` (* (`self.Direction`) -1.0)))
    (:`CastFailed`
      (bind _asmario (cast `/Game/ThirdPersonBP/Blueprints/Mario` OtherActor))
      (if (`/Game/ThirdPersonBP/Blueprints/Mario.HasStarPower` _asmario)
        (`GameplayStatics.PlaySoundAtLocation` "/Game/Audio/Kick_Cue.Kick_Cue" (`self.K2_GetActorLocation` self) (struct) 1.0 1.0 0.0 null null null)
        (`self.Death`)
        (else
          (`/Game/ThirdPersonBP/Blueprints/Mario.TakeDamage` _asmario)
          (`self.StopTortoiseCollisions`)
          (`self.StopGoombaCollisions`)
          (`self.PlantCollisionOff`))))))

(event `PlantCollisionOff`
  ;[1 1 1] Removes collisions of plants
  (bind _outactors (`GameplayStatics.GetAllActorsOfClass` "/Game/Blueprints/Plant_BP.Plant_BP_C"))
  (for _array_element _outactors
    (`PrimitiveComponent.SetCollisionResponseToChannel` (`/Game/Blueprints/Plant_BP.Box` _array_element) "ECC_Pawn" "ECR_Ignore")
    (`KismetSystemLibrary.Delay` 2.0)
    (bind _outactors_2 (`GameplayStatics.GetAllActorsOfClass` "/Game/Blueprints/Plant_BP.Plant_BP_C"))
    (for _array_element_2 _outactors_2
      (`PrimitiveComponent.SetCollisionResponseToChannel` (`/Game/Blueprints/Plant_BP.Box` _array_element_2) "ECC_Pawn" "ECR_Overlap"))))

(event `StopTortoiseCollisions`
  ;[1 1 1] Removes collisions of tortoise
  (bind _outactors (`GameplayStatics.GetAllActorsOfClass` "Tortoise_BP_C"))
  (for _array_element _outactors
    (`PrimitiveComponent.SetCollisionResponseToChannel` (`/Game/Blueprints/Tortoise_BP.DamageCollision` _array_element) "ECC_Pawn" "ECR_Ignore")
    (`PrimitiveComponent.SetCollisionResponseToChannel` (`/Game/Blueprints/Tortoise_BP.SideShell` _array_element) "ECC_Pawn" "ECR_Ignore")
    (`PrimitiveComponent.SetCollisionResponseToChannel` (`/Game/Blueprints/Tortoise_BP.SideShell1` _array_element) "ECC_Pawn" "ECR_Ignore")
    (`PrimitiveComponent.SetCollisionResponseToChannel` (`/Game/Blueprints/Tortoise_BP.TopShell` _array_element) "ECC_Pawn" "ECR_Ignore")
    (`KismetSystemLibrary.Delay` 2.0)
    (bind _outactors_2 (`GameplayStatics.GetAllActorsOfClass` "Tortoise_BP_C"))
    (for _array_element_2 _outactors_2
      (`PrimitiveComponent.SetCollisionResponseToChannel` (`/Game/Blueprints/Tortoise_BP.DamageCollision` _array_element_2) "ECC_Pawn" "ECR_Overlap")
      (`PrimitiveComponent.SetCollisionResponseToChannel` (`/Game/Blueprints/Tortoise_BP.SideShell` _array_element_2) "ECC_Pawn" "ECR_Overlap")
      (`PrimitiveComponent.SetCollisionResponseToChannel` (`/Game/Blueprints/Tortoise_BP.SideShell1` _array_element_2) "ECC_Pawn" "ECR_Overlap")
      (`PrimitiveComponent.SetCollisionResponseToChannel` (`/Game/Blueprints/Tortoise_BP.TopShell` _array_element_2) "ECC_Pawn" "ECR_Block"))))

(event `StopGoombaCollisions`
  ;[1 1 1] Ignore pawn collision for Goomba
  (bind _outactors (`GameplayStatics.GetAllActorsOfClass` "/Game/Blueprints/Goomba_BP.Goomba_BP_C"))
  (for _array_element _outactors
    (`PrimitiveComponent.SetCollisionResponseToChannel` (`/Game/Blueprints/Goomba_BP.DamagePlayerCollision` _array_element) "ECC_Pawn" "ECR_Ignore")
    (`PrimitiveComponent.SetCollisionResponseToChannel` (`/Game/Blueprints/Goomba_BP.DeathCollision` _array_element) "ECC_Pawn" "ECR_Ignore")
    (`KismetSystemLibrary.Delay` 2.0)
    (bind _outactors_2 (`GameplayStatics.GetAllActorsOfClass` "/Game/Blueprints/Goomba_BP.Goomba_BP_C"))
    (for _array_element_2 _outactors_2
      (`PrimitiveComponent.SetCollisionResponseToChannel` (`/Game/Blueprints/Goomba_BP.DamagePlayerCollision` _array_element_2) "ECC_Pawn" "ECR_Overlap")
      (`PrimitiveComponent.SetCollisionResponseToChannel` (`/Game/Blueprints/Goomba_BP.DeathCollision` _array_element_2) "ECC_Pawn" "ECR_Overlap"))))

(event `self.TopShell.OnComponentHit`
  (params (HitComponent :type "PrimitiveComponent Object Reference") (OtherActor :type "Actor Object Reference") (OtherComp :type "PrimitiveComponent Object Reference") (NormalImpulse :type "Vector Structure") (Hit :type "HitResult Structure (by ref)"))
  ;[1 1 1] Shell Collisions
  (cast `/Game/ThirdPersonBP/Blueprints/Mario` OtherActor)
  (if (not (`self.IsShell`))
    (`self.ShellMode`)
    (`self.ShellModeCollision`)))

(event `self.SideShell.OnComponentBeginOverlap`
  (params (OverlappedComponent :type "PrimitiveComponent Object Reference") (OtherActor :type "Actor Object Reference") (OtherComp :type "PrimitiveComponent Object Reference") (OtherBodyIndex :type Integer) (bFromSweep :type Boolean) (SweepResult :type "HitResult Structure (by ref)"))
  ;[1 1 1] Shell Collisions
  (cast `/Game/ThirdPersonBP/Blueprints/Mario` OtherActor)
  (if (`self.IsShell`)
    (set `self.CanMove` true)
    (set `self.Direction` (* (`self.Direction`) -1.0))
    (else
      (`self.ShellMode`)
      (set `self.CanMove` true)))
  (`GameplayStatics.PlaySoundAtLocation` "/Game/Audio/Skid_Cue.Skid_Cue" (`self.K2_GetActorLocation` self) (struct) 1.0 1.0 0.0 null null null :!label _label)
  (`self.DynamicShellCollision`))

(event `ShellModeCollision`
  (bind _damagecollision (`self.DamageCollision`))
  ;[1 1 1] Restricted collisions in (idle) shell mode
  (`PrimitiveComponent.SetCollisionResponseToChannel` _damagecollision "ECC_Pawn" "ECR_Ignore")
  (`KismetSystemLibrary.Delay` (`self.ShellModeDuration`))
  (`PrimitiveComponent.SetCollisionResponseToChannel` _damagecollision "ECC_Pawn" "ECR_Overlap"))

(event `self.SideShell1.OnComponentBeginOverlap`
  (params (OverlappedComponent :type "PrimitiveComponent Object Reference") (OtherActor :type "Actor Object Reference") (OtherComp :type "PrimitiveComponent Object Reference") (OtherBodyIndex :type Integer) (bFromSweep :type Boolean) (SweepResult :type "HitResult Structure (by ref)"))
  ;[1 1 1] Shell Collisions
  (cast `/Game/ThirdPersonBP/Blueprints/Mario` OtherActor)
  (if (`self.IsShell`)
    (set `self.CanMove` true)
    (set `self.Direction` (* (`self.Direction`) -1.0))
    (goto _label)
    (else
      (`self.ShellMode`)
      (set `self.CanMove` true)
      (goto _label))))

(event `DynamicShellCollision`
  ;[1 1 1] Restricted collisions in (dynamic) shell mode
  (`PrimitiveComponent.SetCollisionResponseToChannel` (`self.SideShell1`) "ECC_Pawn" "ECR_Ignore")
  (`PrimitiveComponent.SetCollisionResponseToChannel` (`self.SideShell`) "ECC_Pawn" "ECR_Ignore")
  (`PrimitiveComponent.SetCollisionResponseToChannel` (`self.TopShell`) "ECC_Pawn" "ECR_Ignore")
  (`PrimitiveComponent.SetCollisionResponseToChannel` (`self.DamageCollision`) "ECC_Pawn" "ECR_Ignore")
  (`KismetSystemLibrary.Delay` 0.5)
  (`PrimitiveComponent.SetCollisionResponseToChannel` (`self.DamageCollision`) "ECC_Pawn" "ECR_Overlap")
  (`KismetSystemLibrary.Delay` (`self.ShellModeDuration`))
  (`PrimitiveComponent.SetCollisionResponseToChannel` (`self.SideShell`) "ECC_Pawn" "ECR_Overlap")
  (`PrimitiveComponent.SetCollisionResponseToChannel` (`self.SideShell1`) "ECC_Pawn" "ECR_Overlap")
  (`PrimitiveComponent.SetCollisionResponseToChannel` (`self.TopShell`) "ECC_Pawn" "ECR_Block"))

(fn `Death`
  (`self.K2_DestroyActor`))

(fn `UserConstructionScript`)