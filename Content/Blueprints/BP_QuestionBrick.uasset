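; BP_QuestionBrick is a Mario-style question block that awards a single coin the first time Mario hits it.
; An overlap on its Collider casts the other actor to Mario and checks a HasBeenHit flag.
; The first hit increments Mario's Coins, calls SetMaterial on the Block, sets the flag and plays the coin sound.
; Any later hit only plays a bump sound.
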(event `self.Collider.OnComponentBeginOverlap`
  (params (OverlappedComponent :type "PrimitiveComponent Object Reference") (OtherActor :type "Actor Object Reference") (OtherComp :type "PrimitiveComponent Object Reference") (OtherBodyIndex :type Integer) (bFromSweep :type Boolean) (SweepResult :type "HitResult Structure (by ref)"))
  (bind _asmario (cast `/Game/ThirdPersonBP/Blueprints/Mario` OtherActor))
  (if (`self.HasBeenHit?`)
    (`GameplayStatics.PlaySound2D` "/Game/Audio/Bump.Bump" 1.0 1.0 0.0 null null)
    (else
      (bind _result (`/Engine/EditorBlueprintResources/StandardMacros.IncrementFloat` (`KismetMathLibrary.Conv_IntToDouble` (`/Game/ThirdPersonBP/Blueprints/Mario.Coins` _asmario)))
        (:`  `
          (set `/Game/ThirdPersonBP/Blueprints/Mario.Coins` (`KismetMathLibrary.FTrunc` _result) _asmario)
          (`PrimitiveComponent.SetMaterial` (`self.Block`) 0 null)
          (set `self.HasBeenHit?` true)
          (`GameplayStatics.PlaySound2D` "/Game/Audio/Coin.Coin" 1.0 1.0 0.0 null null))))))

(fn `UserConstructionScript`
  (`parent.UserConstructionScript`))