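; BP_NormalBrick is a brick block that reacts when Mario overlaps its collider.
; The overlap event casts the other actor to Mario and reads its Y scale to decide the outcome.
; A scale above one destroys the brick and plays a break sound, while otherwise only a bump sound plays.
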(event `self.Collider.OnComponentBeginOverlap`
  (params (OverlappedComponent :type "PrimitiveComponent Object Reference") (OtherActor :type "Actor Object Reference") (OtherComp :type "PrimitiveComponent Object Reference") (OtherBodyIndex :type Integer) (bFromSweep :type Boolean) (SweepResult :type "HitResult Structure (by ref)"))
  (bind _asmario (cast `/Game/ThirdPersonBP/Blueprints/Mario` OtherActor))
  (if (> (.y (.scale (`self.GetTransform` _asmario))) 1.0)
    (`self.K2_DestroyActor`)
    (`GameplayStatics.PlaySound2D` "/Game/Audio/Break.Break" 1.0 1.0 0.0 null null)
    (else
      (`GameplayStatics.PlaySound2D` "/Game/Audio/Bump.Bump" 1.0 1.0 0.0 null null))))

(fn `UserConstructionScript`
  (`parent.UserConstructionScript`))