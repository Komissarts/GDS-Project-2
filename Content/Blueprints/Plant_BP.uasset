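; Plant enemy for a Mario-style game that damages Mario when he overlaps its Box, or dies with a kick sound if he has star power.
; A hit also grants brief invulnerability by setting pawn collision to ignore on every plant, Goomba and tortoise found through GetAllActorsOfClass.
; Each of the three events restores its enemy type's collision responses after a short delay, which sits inside the loop body.
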(event `self.Box.OnComponentBeginOverlap`
  (params (OverlappedComponent :type "PrimitiveComponent Object Reference") (OtherActor :type "Actor Object Reference") (OtherComp :type "PrimitiveComponent Object Reference") (OtherBodyIndex :type Integer) (bFromSweep :type Boolean) (SweepResult :type "HitResult Structure (by ref)"))
  ;[1 1 1] Damage player or die
  (bind _asmario (cast `/Game/ThirdPersonBP/Blueprints/Mario` OtherActor))
  (if (`/Game/ThirdPersonBP/Blueprints/Mario.HasStarPower` _asmario)
    (`GameplayStatics.PlaySoundAtLocation` "/Game/Audio/Kick_Cue.Kick_Cue" (`self.K2_GetActorLocation` self) (struct) 1.0 1.0 0.0 null null null)
    (`self.Death`)
    (else
      (`/Game/ThirdPersonBP/Blueprints/Mario.TakeDamage` _asmario)
      (`self.PlantCollisionOff`)
      (`self.StopGoombaCollisions`)
      (`self.StopTortoiseCollisions`))))

(event `PlantCollisionOff`
  ;[1 1 1] Removes collisions of plants
  (bind _outactors (`GameplayStatics.GetAllActorsOfClass` "Plant_BP_C"))
  (for _array_element _outactors
    (`PrimitiveComponent.SetCollisionResponseToChannel` (`/Game/Blueprints/Plant_BP.Box` _array_element) "ECC_Pawn" "ECR_Ignore")
    (`KismetSystemLibrary.Delay` 2.0)
    (bind _outactors_2 (`GameplayStatics.GetAllActorsOfClass` "Plant_BP_C"))
    (for _array_element_2 _outactors_2
      (`PrimitiveComponent.SetCollisionResponseToChannel` (`/Game/Blueprints/Plant_BP.Box` _array_element_2) "ECC_Pawn" "ECR_Overlap"))))

(event `StopGoombaCollisions`
  ;[1 1 1] Ignore pawn collision for Goomba
  (bind _outactors (`GameplayStatics.GetAllActorsOfClass` "/Game/Blueprints/Goomba_BP.Goomba_BP_C"))
  (for _array_element _outactors
    (`PrimitiveComponent.SetCollisionResponseToChannel` (`/Game/Blueprints/Goomba_BP.DamagePlayerCollision` _array_element) "ECC_Pawn" "ECR_Ignore")
    (`PrimitiveComponent.SetCollisionResponseToChannel` (`/Game/Blueprints/Goomba_BP.DeathCollision` _array_element) "ECC_Pawn" "ECR_Ignore")
    (`KismetSystemLibrary.Delay` 2.0)
    (bind _outactors_2 (`GameplayStatics.GetAllActorsOfClass` "/Game/Blueprints/Goomba_BP.Goomba_BP_C"))
    (for _array_element_2 _outactors_2
      (`PrimitiveComponent.SetCollisionResponseToChannel` (`/Game/Blueprints/Goomba_BP.DamagePlayerCollision` _array_element_2) "ECC_Pawn" "ECR_Overlap")
      (`PrimitiveComponent.SetCollisionResponseToChannel` (`/Game/Blueprints/Goomba_BP.DeathCollision` _array_element_2) "ECC_Pawn" "ECR_Overlap"))))

(event `StopTortoiseCollisions`
  ;[1 1 1] Removes collisions of tortoise
  (bind _outactors (`GameplayStatics.GetAllActorsOfClass` "/Game/Blueprints/Tortoise_BP.Tortoise_BP_C"))
  (for _array_element _outactors
    (`PrimitiveComponent.SetCollisionResponseToChannel` (`/Game/Blueprints/Tortoise_BP.DamageCollision` _array_element) "ECC_Pawn" "ECR_Ignore")
    (`PrimitiveComponent.SetCollisionResponseToChannel` (`/Game/Blueprints/Tortoise_BP.SideShell` _array_element) "ECC_Pawn" "ECR_Ignore")
    (`PrimitiveComponent.SetCollisionResponseToChannel` (`/Game/Blueprints/Tortoise_BP.SideShell1` _array_element) "ECC_Pawn" "ECR_Ignore")
    (`PrimitiveComponent.SetCollisionResponseToChannel` (`/Game/Blueprints/Tortoise_BP.TopShell` _array_element) "ECC_Pawn" "ECR_Ignore")
    (`KismetSystemLibrary.Delay` 2.0)
    (bind _outactors_2 (`GameplayStatics.GetAllActorsOfClass` "/Game/Blueprints/Tortoise_BP.Tortoise_BP_C"))
    (for _array_element_2 _outactors_2
      (`PrimitiveComponent.SetCollisionResponseToChannel` (`/Game/Blueprints/Tortoise_BP.DamageCollision` _array_element_2) "ECC_Pawn" "ECR_Overlap")
      (`PrimitiveComponent.SetCollisionResponseToChannel` (`/Game/Blueprints/Tortoise_BP.SideShell` _array_element_2) "ECC_Pawn" "ECR_Overlap")
      (`PrimitiveComponent.SetCollisionResponseToChannel` (`/Game/Blueprints/Tortoise_BP.SideShell1` _array_element_2) "ECC_Pawn" "ECR_Overlap")
      (`PrimitiveComponent.SetCollisionResponseToChannel` (`/Game/Blueprints/Tortoise_BP.TopShell` _array_element_2) "ECC_Pawn" "ECR_Block"))))

(fn `Death`
  (`self.K2_DestroyActor`))

(fn `UserConstructionScript`)