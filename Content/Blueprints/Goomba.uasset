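; Goomba actor that travels along the spline of a referenced track, starting when play begins.
; A timeline, with play rate set from Duration and start time from StartOffset, drives an alpha from which distance along the spline is interpolated.
; Each update sets the actor's world location and rotation from the spline at that distance.
; The FinishedPath flag logic is unconnected and never runs.
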(event `self.ReceiveBeginPlay`
  (`self.MoveOnSpline`))

(event `MoveOnSpline`
  (bind _movealong (`self.MoveAlong`))
  (bind _trackspline (`/Game/Blueprints/Track_BP.TrackSpline` (`self.TrackRef`)))
  (bind _returnvalue (`KismetMathLibrary.Lerp` 0.0 (`SplineComponent.GetSplineLength` _trackspline) (`self.Alpha`)))
  (`TimelineComponent.SetPlayRate` _movealong (/ 1.0 (`self.Duration`)))
  (`TimelineComponent.SetNewTime` _movealong (`self.StartOffset`))
  (bind (_direction _alpha) (`Timeline|MoveAlong`)
    (:`Update`
      (set `self.Alpha` _alpha)
      (`self.K2_SetActorLocationAndRotation` (`SplineComponent.GetLocationAtDistanceAlongSpline` _trackspline _returnvalue "World") (`SplineComponent.GetRotationAtDistanceAlongSpline` _trackspline _returnvalue "World")))))

(fn `UserConstructionScript`)